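; Rifle bullet projectile that damages what its box collision hits, then spawns a small impact effect and destroys itself.
; Physics-simulating components also receive a velocity-based impulse, while non-simulating hits on the owner are ignored.
; Damage uses the rifle damage type and prints a debug string at the hit.
; Projectile stop also triggers the impact effect, while Tick destroys the bullet without it when the shell mesh's physics speed is below a threshold.
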(event `self.ProjectileMovement.OnProjectileStop`
  (params (ImpactResult :type "HitResult Structure (by ref)"))
  (`NiagaraFunctionLibrary.SpawnSystemAtLocation` "/Game/GameCreatedContent/Weapons/Rifle/Bullet/FXS_Rifle_Bullet_Impact.FXS_Rifle_Bullet_Impact" (`self.K2_GetActorLocation`) (`self.K2_GetActorRotation`) (0.25 0.25 0.25) :!label _label)
  (`self.K2_DestroyActor` :!label _label_2))

(event `self.Box.OnComponentHit`
  (params (HitComponent :type "PrimitiveComponent Object Reference") (OtherActor :type "Actor Object Reference") (OtherComp :type "PrimitiveComponent Object Reference") (NormalImpulse :type "Vector Structure") (Hit :type "HitResult Structure (by ref)"))
  (if (`SceneComponent.IsSimulatingPhysics` OtherComp "None")
    (`PrimitiveComponent.AddImpulse` OtherComp (* (`MovementComponent.Velocity` (`self.ProjectileMovement`)) 1.0) "None" false)
    (bind _returnvalue (`GameplayStatics.ApplyDamage` OtherActor (`self.BaseDamage`) (`self.GetInstigatorController`) (`self.GetOwner`) "/Game/GameCreatedContent/Weapons/Rifle/Bullet/BP_Rifle_DamageType.BP_Rifle_DamageType_C" :!label _label_3))
    (`KismetSystemLibrary.DrawDebugString` (`self.K2_GetActorLocation`) (`KismetStringLibrary.Concat_StrStr` "Collided with " (`KismetSystemLibrary.GetDisplayName` OtherComp) " of " (`KismetSystemLibrary.GetDisplayName` OtherActor) " for " (`KismetStringLibrary.Conv_DoubleToString` _returnvalue) "damage") null (struct :`R` 1.0 :`G` 1.0 :`B` 1.0 :`A` 1.0) 0.5)
    (goto _label)
    (elif (not (== OtherActor (`self.GetOwner`)))
      (goto _label_3))))

(event `self.ReceiveTick`
  (params (DeltaSeconds :type "Float (single-precision)"))
  (bind _returnvalue (`PrimitiveComponent.GetPhysicsLinearVelocity` (`self.SM_Shell_556x45`) "None"))
  (if (< (`KismetMathLibrary.VSize` _returnvalue) 7000.0)
    (goto _label_2)))

(fn `UserConstructionScript`)